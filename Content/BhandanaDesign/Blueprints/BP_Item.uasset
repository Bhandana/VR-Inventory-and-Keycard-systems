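; BP_Item is a VR pickup that a motion controller grabs and drops, either into inventory slots or back into the physics world.
; While held, overlaps with actors tagged Inventory query the slot by item type and remember a valid one.
; Drop attaches the item to that slot with an inventory rotation offset and assigns it, falling back to a physics drop if refused.
; Pickup notifies the previous slot, and absolute model scale keeps slots from resizing it.
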(event OnComponentBeginOverlap(Model)
  (params (OverlappedComponent :type Primitive%20Component%20Object%20Reference) (OtherActor :type Actor%20Object%20Reference) (OtherComp :type Primitive%20Component%20Object%20Reference) (OtherBodyIndex :type Integer) (bFromSweep :type Boolean) (SweepResult :type Hit%20Result%20Structure%20%28by%20ref%29))
  ;[0.07996 0.1053 0.2865] Stores the Actor in memory if it's an inventory slot, and checks if the item can go there
  (if (and (Actor|ActorHasTag OtherActor "Inventory") (Variables|Default|GetVAR_IsHeld))
    (bind _allowed_in_slot_ (Class|BPIInventorySystem|InformInventorySlot(Message) OtherActor (Variables|ItemStats|GetItemType) self))
    (if _allowed_in_slot_
      (Variables|Default|SetActorReference OtherActor))))

(event OnComponentEndOverlap(Model)
  (params (OverlappedComponent :type Primitive%20Component%20Object%20Reference) (OtherActor :type Actor%20Object%20Reference) (OtherComp :type Primitive%20Component%20Object%20Reference) (OtherBodyIndex :type Integer))
  ;[0.07996 0.1053 0.2865] Clears the reference of which slot this item is overlapping, when it leaves that slot's area
  (if (Actor|ActorHasTag OtherActor "Inventory")
    (bind _allowed_in_slot_ (Class|BPIInventorySystem|InformInventorySlot(Message) OtherActor (Variables|ItemStats|GetItemType)))
    (if (and _allowed_in_slot_ (== (Variables|Default|GetActorReference) OtherActor))
      (Variables|Default|SetActorReference 0))))

(event Custom|ManualDrop
  ;[0.07996 0.1053 0.2865] Drops the item, putting it into a slot if it's intended to into one.
  (Physics|SetSimulatePhysics (Variables|Default|GetModel) true)
  (Transformation|DetachFromActor "KeepWorld" "KeepWorld" "KeepWorld")
  (Collision|SetCollisionResponsetoChannel (Variables|Default|GetModel) "ECC_Visibility" "ECR_Block")
  (Collision|SetCollisionEnabled (Variables|Default|GetModel) "QueryAndPhysics")
  (Variables|Default|SetActorReference 0))

(event EventBeginPlay
  ;[0.07996 0.1053 0.2865] Begin Play -- Sets the scale to Absolute to inventory slots don't mess with it
  (Transformation|SetAbsolute (Variables|Default|GetModel) false false true))

(event EventPickup
  (params (AttachTo :type Scene%20Component%20Object%20Reference))
  (bind _var_issnaptotarget (Variables|ItemStats|GrabSettings|GetVAR_IsSnapToTarget))
  (bind _returnvalue (select _var_issnaptotarget "SnapToTarget" "KeepWorld"))
  ;[0.07996 0.1053 0.2865] Attaches the actor to the hand that grabbed it; Updates the inventory slot it came from (if it did)
  (Variables|Default|SetVAR_IsHeld true)
  (Utilities|IsValid (Variables|Default|GetActorReferenceMemory)
    (:Is%20Valid
      (Class|BPIInventorySystem|AssignItem(Message) (Variables|Default|GetActorReferenceMemory) (Variables|ItemStats|GetItemType))
      (Variables|Default|SetActorReferenceMemory 0))
    (:Is%20Not%20Valid
      _))
  (Physics|SetSimulatePhysics (Variables|Default|GetModel) false)
  (Transformation|AttachComponentToComponent (VehicleSound|GetRootComponent) AttachTo "None" _returnvalue _returnvalue "KeepWorld" false)
  (Collision|SetCollisionResponsetoChannel (Variables|Default|GetModel) "ECC_Visibility" "ECR_Ignore"))

(event EventDrop
  (bind _model (Variables|Default|GetModel))
  ;[0.07996 0.1053 0.2865] Drops the item, putting it into a slot if it's intended to into one.
  (Variables|Default|SetVAR_IsHeld false)
  (Utilities|IsValid (Variables|Default|GetActorReference)
    (:Is%20Valid
      (Transformation|AttachComponentToComponent (VehicleSound|GetRootComponent) (Variables|/Script/Engine.Actor|GetRootComponent (Variables|Default|GetActorReference)) "None" "SnapToTarget" "SnapToTarget" "KeepWorld" false)
      (Transformation|AddActorLocalRotation (Variables|/Script/Engine.SceneComponent|GetRelativeRotation (Variables|Default|GetInventoryRotation)) false false)
      (Variables|Default|SetActorReferenceMemory (Variables|Default|GetActorReference))
      (bind _allowed_in_slot_ (Class|BPIInventorySystem|AssignItem(Message) (Variables|Default|GetActorReference) (Variables|ItemStats|GetItemType) self))
      (if _allowed_in_slot_
        (Collision|SetCollisionResponsetoChannel _model "ECC_Visibility" "ECR_Ignore")
        (Collision|SetCollisionEnabled _model "QueryOnly")
        (else
          (CallFunction|ManualDrop)
          (Variables|Default|SetActorReferenceMemory 0))))
    (:Is%20Not%20Valid
      (Physics|SetSimulatePhysics (Variables|Default|GetModel) true)
      (Transformation|DetachFromActor "KeepWorld" "KeepWorld" "KeepWorld")
      (Collision|SetCollisionResponsetoChannel (Variables|Default|GetModel) "ECC_Visibility" "ECR_Block")
      (Collision|SetCollisionEnabled (Variables|Default|GetModel) "QueryAndPhysics")
      (Variables|Default|SetActorReference 0))))

(fn ConstructionScript)