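; BP_Item_VRPistol is a VR pistol item that fires a hitscan shot when used.
; Its Use event runs a visibility line trace from the model's FirePoint socket along the actor's forward vector, ignoring the owner of the model's attach parent.
; A hit applies a small fixed amount of damage to the struck actor, and the trace is drawn as timed debug lines.
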(event EventBeginPlay
  (|CallParentFunction) ; This node is disabled and will not be called.\nDrag off pins to build functionality.
)

(event Collision|EventActorBeginOverlap
  (params (OtherActor :type Actor%20Object%20Reference))
  (|CallParentFunction OtherActor) ; This node is disabled and will not be called.\nDrag off pins to build functionality.
)

(event EventTick
  (params (DeltaSeconds :type Float%20%28single-precision%29))
  (|CallParentFunction DeltaSeconds) ; This node is disabled and will not be called.\nDrag off pins to build functionality.
)

(event EventUse
  (bind _model (Variables|Default|GetModel))
  (bind _returnvalue (Transformation|GetSocketLocation _model "FirePoint"))
  ;[0.07996 0.1053 0.2865] Linetraces for a hit, if there is one; deals some damage to the actor that was hit
  (bind (_outhit _returnvalue_2) (Collision|LineTraceByChannel _returnvalue (+ _returnvalue (* (Transformation|GetActorForwardVector) 5e+03)) "TraceTypeQuery1" false (Utilities|Array|MakeArray (Components|GetOwner (Transformation|GetAttachParent (Variables|Default|GetModel)))) "ForDuration"))
  (if _returnvalue_2
    (Game|Damage|ApplyDamage (.HitActor (Collision|BreakHitResult _outhit)) 2.0 0 0 "/Script/Engine.DamageType")))

(fn ConstructionScript
  (|CallParentFunction))